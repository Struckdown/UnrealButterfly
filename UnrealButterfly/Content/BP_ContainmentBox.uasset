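; BP_ContainmentBox is a volume that keeps Boid actors inside its bounds by wrapping them to the opposite side when they leave.
; BeginPlay binds an end-overlap handler, which ignores any actor that is not a Boid.
; For each axis where the boid lies beyond the collision component's box extent, the handler mirrors its position through the box's actor location.
; The boid moves there without sweep, and other axes stay unchanged.
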(event `self.ReceiveBeginPlay`
  (add `self.OnActorEndOverlap` (delegate `OnActorEndOverlap_Event`)))

(event `OnActorEndOverlap_Event` :!signature `self.OnActorEndOverlap`
  (params (OverlappedActor :type "Actor Object Reference") (OtherActor :type "Actor Object Reference"))
  (bind _returnvalue (`self.K2_GetActorLocation` OtherActor))
  (bind _returnvalue_2 (`self.K2_GetActorLocation` OverlappedActor))
  (bind (_x _y _z) (`KismetMathLibrary.BreakVector3f` _returnvalue))
  (bind (_x_2 _y_2 _z_2) (`KismetMathLibrary.BreakVector3f` _returnvalue_2))
  (bind (_x_3 _y_3 _z_3) (`KismetMathLibrary.BreakVector3f` _returnvalue))
  (bind (_x_4 _y_4 _z_4) (`KismetMathLibrary.BreakVector3f` (`.BoxExtent` (`KismetSystemLibrary.GetComponentBounds` (`self.CollisionComponent`)))))
  (bind _asboid (cast `Boid` OtherActor))
  (`self.K2_SetActorLocation` _asboid (`KismetMathLibrary.MakeVector` (select `bool` (> (`KismetMathLibrary.Abs` (- _x_2 _x)) _x_4) :`false` _x_3 :`true` (.x (- _returnvalue (* (- _returnvalue _returnvalue_2) 2.0))) :!type "Float (double-precision)") (select `bool` (> (`KismetMathLibrary.Abs` (- _y_2 _y)) _y_4) :`false` _y_3 :`true` (.y (- _returnvalue (* (- _returnvalue _returnvalue_2) 2.0))) :!type "Float (double-precision)") (select `bool` (> (`KismetMathLibrary.Abs` (- _z_2 _z)) _z_4) :`false` _z_3 :`true` (.z (- _returnvalue (* (- _returnvalue _returnvalue_2) 2.0))) :!type "Float (double-precision)")) false false))

(fn `UserConstructionScript`)